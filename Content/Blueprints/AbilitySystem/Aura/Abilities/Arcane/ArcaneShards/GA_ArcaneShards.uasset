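; Arcane Shards gameplay ability that shows a magic circle, then casts a series of shards at the clicked location.
; On input press it spawns a BP_PointCollection for randomly rotated ground points, faces the target and plays the cast montage.
; The montage event hides the circle and starts a looping timer that fires a gameplay cue and radial damage with upward, outward knockback at each successive point.
; After the last shard it destroys the collection and ends.
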(event `self.K2_ActivateAbility`
  (`|ExecutionSequence`
    (:`then_0`
      (message `PlayerInterface.ShowMagicCircle` (`self.GetAvatarActorFromActorInfo`) null))
    (:`then_1`
      (`AbilityTask_WaitInputPress.WaitInputPress` false
        (:`OnPress`
          (bind (_asynctaskproxy _datahandle) (`TargetDataUnderMouse.CreateTargetDataUnderMouse`)
            (:`ValidData`
              (bind _output_get (set `self.MouseHitLocation` (`.ImpactPoint` (`GameplayStatics.BreakHitResult` (`AbilitySystemBlueprintLibrary.GetHitResultFromTargetData` _datahandle)))))
              (bind _returnvalue (`|SpawnActorFromClass` "/Game/Blueprints/AbilitySystem/Aura/Abilities/Arcane/ArcaneShards/BP_PointCollection.BP_PointCollection_C" (`KismetMathLibrary.MakeTransform` _output_get) "AlwaysSpawn" "MultiplyWithRoot" null null))
              (bind _output_get_2 (set `self.PointCollection` _returnvalue))
              (set `self.GroundPoints` (`PointCollection.GetGroundPoints` _output_get_2 (`self.MouseHitLocation`) 0 (`KismetMathLibrary.RandomFloatInRange` 0.0 360.0)))
              (message `CombatInterface.UpdateFacingTarget` (`self.GetAvatarActorFromActorInfo`) (`self.MouseHitLocation`))
              (`AbilityTask_PlayMontageAndWait.CreatePlayMontageAndWaitProxy` "None" "/Game/Assets/Characters/Aura/Animations/Abilities/AM_CastArcaneShards.AM_CastArcaneShards" 1.0 "None" false
                (:`then`
                  (`AbilityTask_WaitGameplayEvent.WaitGameplayEvent` (struct :`TagName` "Event.Montage.ArcaneShards") null
                    (:`EventReceived`
                      (bind _returnvalue_2 (`KismetSystemLibrary.K2_SetTimerDelegate` (delegate `SpawnShard`) (`self.ShardSpawnDelta`) true))
                      (set `self.ShardSpawnTimer` _returnvalue_2)
                      (`self.SpawnShard`)
                      (message `PlayerInterface.HideMagicCircle` (`self.GetAvatarActorFromActorInfo`)))))))))))))

(event `SpawnShard`
  (if (< (`self.Count`) (`self.MaxNumShards`))
    (`self.StoreShardSpawnLocation`)
    (`self.StoreActorsToDamage`)
    (for _array_element (`self.ActorsToDamage`)
      (`self.RadialDamageToActor` _array_element))
    (`/Engine/EditorBlueprintResources/StandardMacros.IncrementInt` (`self.Count`)
      (:`  `
        (`self.K2_ExecuteGameplayCueWithParams` (struct :`TagName` "GameplayCue.ArcaneShards") (`AbilitySystemBlueprintLibrary.MakeGameplayCueParameters` 0.0 0.0 (struct) (struct) (struct) (struct) (struct) (`self.ShardSpawnLocation`)))))
    (else
      (`KismetSystemLibrary.K2_ClearAndInvalidateTimerHandle` (`self.ShardSpawnTimer`))
      (`KismetSystemLibrary.Delay` 0.2)
      (`Actor.K2_DestroyActor` (`self.PointCollection`))
      (`self.K2_EndAbility`))))

(fn `RadialDamageToActor`
  (params (TargetActor :type "Actor Object Reference"))
  (bind _returnvalue (- (`Actor.K2_GetActorLocation` TargetActor) (`self.ShardSpawnLocation`)))
  (`AuraAbilitySystemLibrary.ApplyDamageEffect` (`self.MakeDamageEffectParamsFromClassDefaults` TargetActor (`self.ShardSpawnLocation`) true _returnvalue true _returnvalue true 35.0)))

(fn `StoreActorsToDamage`
  (bind _returnvalue (`self.GetAvatarActorFromActorInfo`))
  (bind _outoverlappingactors (`AuraAbilitySystemLibrary.GetLivePlayersWithinRadius` _returnvalue (`|MakeArray` _returnvalue) (`self.RadialDamageOuterRadius`) (`self.ShardSpawnLocation`)))
  (set `self.ActorsToDamage` _outoverlappingactors))

(fn `StoreShardSpawnLocation`
  (set `self.ShardSpawnLocation` (`SceneComponent.K2_GetComponentLocation` (`|GetArrayItem` (`self.GroundPoints`) (`self.Count`)))))